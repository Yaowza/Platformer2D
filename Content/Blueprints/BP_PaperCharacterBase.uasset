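; Paper2D side-scroller player character with movement, jumping, pause, health and melon collection.
; Movement input refreshes a state-driven flipbook (idle, run, jump, fall, hurt) and flips facing through control rotation.
; Capsule hits on enemies use hit direction to damage a stomped enemy or hurt the player, with knockback and a short DoOnce debounce.
; Damage routes through a health component; event dispatchers announce health changes, death, melons remaining and all melons collected.
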(event OnComponentHit(CapsuleComponent)
  (params (HitComponent :type Primitive%20Component%20Object%20Reference) (OtherActor :type Actor%20Object%20Reference) (OtherComp :type Primitive%20Component%20Object%20Reference) (NormalImpulse :type Vector :default "0, 0, 0") (Hit :type Hit%20Result%20Structure%20%28by%20ref%29))
  (bind _asbp_enemy_base (Utilities|Casting|CastToBP_EnemyBase OtherActor))
  (Variables|Default|SetHitEnemyRef _asbp_enemy_base)
  (Utilities|FlowControl|DoOnce false
    (:Completed
      (Variables|Default|SetHitDirection (Math|Vector|Normalize (- (.location Hit) (Transformation|GetActorLocation)) 0.0))
      (Utilities|FlowControl|Sequence
        (:then_0
          ;[0 0 0] détection du sens de la collision (est ce que l'on touche par le dessus ?)
          (if (<= (.z (Variables|Default|GetHitDirection)) -0.75)
            ;[0 0 0] Si oui, on applique les dégats à l'ennemi
            (Game|Damage|ApplyDamage (Variables|Default|GetHitEnemyRef) (Variables|Default|GetjumpDamage) 0 0)
            ;[0 0 0] knock back
            (Components|Movement|StopMovementImmediately (Variables|Character|GetCharacterMovement))
            (Physics|AddImpulse (Variables|Character|GetCharacterMovement) (Math|Vector|MakeVector 0.0 0.0 4.5e+02) true)
            ;;[1 0.1269 0.916] play sfx
            (CallFunction|PlaySfx "/Game/Assets/Sounds/jump_1.jump_1" 0.0)
            (else
              ;;[0 0 0] si non, on applique au joueur
              (Game|Damage|ApplyDamage self 25.0 0 0)
              (Components|Movement|StopMovementImmediately (Variables|Character|GetCharacterMovement))
              (if (not false)
                (Physics|AddImpulse (Variables|Character|GetCharacterMovement) (Math|Vector|MakeVector (* (.x (Variables|Default|GetHitDirection)) (* -1.0 4.5e+02)) 0.0 1.5e+02) true)))))
        (:then_1
          (Utilities|FlowControl|Delay 0.1)
          (CallFunction|ResetHit))))))

(event Custom|resetHit
  (Utilities|FlowControl|DoOnce false) ; enters at Reset
)

(event EventBeginPlay
  ;[0 0 0] Initialisation ( notes : heal du perso dans le construct )
  (CallFunction|UpdateFlipBook)
  (bind _outactors (Actor|GetAllActorsOfClass "/Game/Blueprints/Items/BP_HealthCollectible.BP_HealthCollectible_C"))
  (Variables|Default|SettotalMelon (Utilities|Array|Length _outactors))
  (CallFunction|CallMelonHudUpdate))

(event Game|Damage|EventAnyDamage
  (params (Damage :type Float%20%28single-precision%29) (DamageType :type Damage%20Type%20Object%20Reference) (InstigatedBy :type Controller%20Object%20Reference) (DamageCauser :type Actor%20Object%20Reference))
  ;[0 0 0] On applique si le joueur est vivant
  (Utilities|IfIsAlive)
  ;[0 0 0] Take damage
  (Default|DoDamage (Variables|Default|GetBPC_HealthComponent) Damage)
  ;[0 0 0] Death/Hurt, on envoi un message de notif
  (if (Default|GetIsDead (Variables|Default|GetBPC_HealthComponent))
    (CallFunction|PlayerUnspawn)
    (Default|CallPlayerDiedEventDispatcher)
    (else
      ;;[0 0 0] Si les degats sont positifs on passe en state "hurt" sinon c'est un "heal"
      (if (< Damage 0.0)
        (Default|CallPlayerHealthChangedEventDispatcher)
        (else
          (Variables|Default|SethurtState true)
          ;;;[1 0.1063 0.8399] sfx
          (CallFunction|PlaySfx "/Game/Assets/Sounds/HitHurt_2.HitHurt_2" 0.0)
          (Default|CallPlayerHealthChangedEventDispatcher)
          (Utilities|FlowControl|Delay 0.5)
          (Variables|Default|SethurtState false))))))

(event Input|ActionEvents|InputActionJump
  (params (Key :type Key%20Structure :default "None"))
  ;[0 0 0] Character movement : Jump
  (:Pressed
    (Utilities|IfIsAlive)
    (if (Character|CanJump)
      (Character|Jump)
      (CallFunction|PlaySfx "/Game/Assets/Sounds/jump_1.jump_1" 0.0)))
  (:Released
    (Utilities|IfIsAlive)
    (Character|StopJumping)))

(event Input|ActionEvents|InputActionPause
  (params (Key :type Key%20Structure :default "None"))
  (:Pressed
    (Game|SetGamePaused (not (Game|IsGamePaused)))))

(event Input|AxisEvents|InputAxisMoveForward
  (params (AxisValue :type Float%20%28single-precision%29))
  ;[0 0 0] Character movement : Move Forward
  (Utilities|IfIsAlive)
  (Pawn|Input|AddMovementInput "1.000000, 0, 0" AxisValue false)
  (CallFunction|UpdateFlipBook))

(fn ConstructionScript)

(fn UpdateFlipBook
  ;[0 0 0] Update "StateMachine"
  (Variables|Default|SetMyPlayerState (select (Variables|Default|GethurtState) "NewEnumerator4" (select (!= (Math|Vector|VectorLength (Transformation|GetVelocity)) 0.0) (select (AI|Components|NavMovement|IsFalling (Variables|Character|GetCharacterMovement)) (select (<= (.z (Transformation|GetVelocity)) 0.0) "NewEnumerator3" "NewEnumerator2") "NewEnumerator1") "NewEnumerator0")))
  ;[0 0 0] Update Sprite flipbook
  (Sprite|SetFlipbook (Variables|Default|GetSprite) (Utilities|Select :Index (Variables|Default|GetMyPlayerState) :NewEnumerator0 "/Game/Blueprints/sus/idle_red.idle_red" :NewEnumerator1 "/Game/Blueprints/sus/walk_red.walk_red" :NewEnumerator2 "/Game/Blueprints/sus/jump2_red.jump2_red" :NewEnumerator3 "/Game/Blueprints/sus/fall_red.fall_red" :NewEnumerator4 "/Game/Blueprints/sus/dmg_red.dmg_red"))
  ;[0 0 0] Update rotation
  (CallFunction|UpdateFlipBookRotation))

(fn UpdateFlipBookRotation
  (Math|Float|CompareFloat (.x (Transformation|GetVelocity)) 0.0
    (:>
      (Pawn|SetControlRotation (Game|GetPlayerController 0) (Math|Rotator|MakeRotator 0.0 0.0 0.0)))
    (:<
      (Pawn|SetControlRotation (Game|GetPlayerController 0) (Math|Rotator|MakeRotator 0.0 0.0 1.8e+02)))))

(fn PlayerUnspawn
  (Components|Movement|StopMovementImmediately (Variables|Character|GetCharacterMovement))
  (Variables|/Script/Engine.CharacterMovementComponent|SetGravityScale (Variables|Character|GetCharacterMovement) 0.0)
  (Sprite|SetFlipbook (Variables|Default|GetSprite) "/Game/Blueprints/sus/dead_red.dead_red")
  (Components|Timeline|SetLooping (Variables|Default|GetSprite) false))

(fn PlayerSpawn
  (Variables|/Script/Engine.CharacterMovementComponent|SetGravityScale (Variables|Character|GetCharacterMovement) 2.0)
  (Sprite|SetFlipbook (Variables|Default|GetSprite) "/Game/Assets/Flipbooks/FB-ninja-frog-Idle.FB-ninja-frog-Idle")
  (Components|Timeline|SetLooping (Variables|Default|GetSprite) true)
  (Components|Timeline|PlayfromStart (Variables|Default|GetSprite)))

(fn CallMelonHudUpdate
  (Default|CallMelonCollectorEventDistacher (- (Variables|Default|GettotalMelon) (Variables|Default|GetmelonCollectedCounter))))

(fn CollectMelon
  (bind _result (Math|Integer|IncrementInt (Variables|Default|GetmelonCollectedCounter))
    (:%20%20
      (Default|CallMelonCollectorEventDistacher (- (Variables|Default|GettotalMelon) _result))
      (if (>= (Variables|Default|GetmelonCollectedCounter) (Variables|Default|GettotalMelon))
        (Default|CallAllMelonsCollectedEventDispatcher)))))